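; BP_AI_Base is an AI base Blueprint that supplies a looping sequence of points to move to.
; GetNextPoint increments CurrentMoveIndex, resets it to zero when the modulo against the PointsToMove length is zero, and returns the point at that index.
; The event graph and construction script are empty, so the movement itself is not handled in this file.
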(event EventBeginPlay)

(event Collision|EventActorBeginOverlap
  (params (OtherActor :type Actor%20Object%20Reference)))

(event EventTick
  (params (DeltaSeconds :type Float%20%28single-precision%29)))

(fn ConstructionScript)

(fn GetNextPoint
  (bind _result (Math|Integer|IncrementInt (Variables|Default|GetCurrentMoveIndex))
    (:%20%20
      (if (== (Math|Integer|%(Integer) _result (Utilities|Array|Length (Variables|Default|GetPointsToMove))) 0)
        (bind _output_get (Variables|Default|SetCurrentMoveIndex 0))
        (return (Utilities|Array|Get(acopy) (Variables|Default|GetPointsToMove) _output_get))
        (else
          (return (Utilities|Array|Get(acopy) (Variables|Default|GetPointsToMove) (Variables|Default|GetCurrentMoveIndex))))))))