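; BP_AISpawner is a placed actor that spawns an AI actor of a configurable class at its own location when play begins.
; ConvertToWorld transforms the MovePoints array from the spawner's local space into world space using its actor transform.
; The resulting points are passed to the spawned actor as PointsToMove on spawn, giving it a path relative to where the spawner sits.
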(event EventBeginPlay
  (bind _locationsinworld (CallFunction|ConverttoWorld))
  (Game|SpawnActorfromClass (Variables|Default|GetSpawnerClass) (Math|Transform|MakeTransform (Transformation|GetActorLocation) "0, 0, 0" "1.000000,1.000000,1.000000") "Undefined" 0 _locationsinworld 0))

(event Collision|EventActorBeginOverlap
  (params (OtherActor :type Actor%20Object%20Reference)))

(event EventTick
  (params (DeltaSeconds :type Float%20%28single-precision%29)))

(fn ConstructionScript)

(fn ConverttoWorld
  (LocalVariables|SetActorTransform (Transformation|GetActorTransform))
  (for _array_element (Variables|Default|GetMovePoints)
    (Utilities|Array|Add (LocalVariables|GetInWorld) (Math|Transform|TransformLocation (LocalVariables|GetActorTransform) _array_element)))
  (return (LocalVariables|GetInWorld)))