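; Game mode that acts as a hub between an attributes actor and a list of linked listener actors.
; It stores the registered attributes actor, binds an event to its attribute changes, and exposes a getter with a validity flag.
; Linked actors register uniquely into an array.
; SendTheMessage passes a parameter to each through ChangeLocalAttributesMessage, looping in reverse to safely prune invalid entries.
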(event EventBeginPlay)

(event EventTick
  (params (DeltaSeconds :type Float%20%28single-precision%29)))

(event EventSetLinkAttributesActor
  (params (ActorWithParams :type BP%20Actor%20with%20Params%20Object%20Reference))
  (bind _output_get (Variables|Default|SetActorWithParams ActorWithParams))
  (EventDispatchers|BindEventtoOnAttributesChanges _output_get (EventDispatchers|CreateEvent :!event SendtheMessage)))

(event EventAddActortoLinkedArray
  (params (NewActor :type Actor%20Object%20Reference))
  (Utilities|Array|AddUnique (Variables|Default|GetActorToCall) NewActor))

(fn ConstructionScript)

(fn SendtheMessage
  (params (NewParam :type S%20Actor%20Attributes%20Structure))
  (bind (_arrayindex _arrayelement) (Utilities|Array|ReverseforEachLoop (Variables|Default|GetActorToCall))
    (:LoopBody
      (LocalVariables|SetLoc_Index _arrayindex)
      (if (Utilities|IsValid _arrayelement)
        (Class|BPIChanges|ChangeLocalAttributes(Message) _arrayelement NewParam)
        (else
          (Utilities|Array|RemoveIndex (Variables|Default|GetActorToCall) (LocalVariables|GetLoc_Index)))))
    (:Completed
      (return))))

(fn GetLinkAttributesActor
  (bind _actorwithparams (Variables|Default|GetActorWithParams))
  (return _actorwithparams (Utilities|IsValid _actorwithparams)))