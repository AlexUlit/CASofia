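; BP_ActorWithParams is a task Actor that holds an SActorAttributes struct and broadcasts it through the OnAttributesChanges event dispatcher.
; On BeginPlay it passes itself to the GameMode via a SetLinkAttributesActor message.
; After a delay it modifies Damage and broadcasts, then broadcasts Attributes again after a second delay.
; A Debug function, not called within this Blueprint, prints Health, Stamina, Damage and SomeCondition from a passed struct.
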(event EventBeginPlay
  (Class|BPIParams|SetLinkAttributesActor(Message) (Game|GetGameMode) self)
  (Utilities|FlowControl|Delay 2.0)
  (bind _structout (Utilities|Struct|SetmembersinSActorAttributes (Variables|Default|GetAttributes) 1e+02))
  (Default|CallOnAttributesChanges _structout)
  (Utilities|FlowControl|Delay 2.0)
  (Default|CallOnAttributesChanges (Variables|Default|GetAttributes)))

(event Collision|EventActorBeginOverlap
  (params (OtherActor :type Actor%20Object%20Reference)))

(event EventTick
  (params (DeltaSeconds :type Float%20%28single-precision%29)))

(fn ConstructionScript)

(fn Debug
  (params (NewParam4 :type S%20Actor%20Attributes%20Structure))
  (bind (_health _stamina _damage _somecondition) (Utilities|Struct|BreakSActorAttributes NewParam4))
  (Development|PrintString (Utilities|String|ToString(Float) _health))
  (Development|PrintString (Utilities|String|ToString(Float) _stamina))
  (Development|PrintString (Utilities|String|ToString(Float) _damage))
  (Development|PrintString (Utilities|String|ToString(Boolean) _somecondition)))