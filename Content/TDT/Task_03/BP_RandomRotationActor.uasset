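; BP_RandomRotationActor is a static mesh actor that varies its own size and heading at construction for visual variety.
; The construction script gives the mesh a random world scale, drawing each axis independently from its own min/max variables.
; It then sets a random world yaw over a full turn while keeping the current roll and pitch.
; The event graph holds no active logic.
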(event EventBeginPlay)

(event Collision|EventActorBeginOverlap
  (params (OtherActor :type Actor%20Object%20Reference)))

(event EventTick
  (params (DeltaSeconds :type Float%20%28single-precision%29)))

(fn ConstructionScript
  (bind _staticmesh (Variables|Default|GetStaticMesh))
  (bind _returnvalue (Transformation|GetWorldRotation _staticmesh))
  (Transformation|SetWorldScale3D (Variables|Default|GetStaticMesh) (Math|Vector|MakeVector (Math|Random|RandomFloatinRange (Variables|Settings|Scale|Min|GetScale_X_Min) (Variables|Settings|Scale|Max|GetScale_X_Max)) (Math|Random|RandomFloatinRange (Variables|Settings|Scale|Min|GetScale_Y_Min) (Variables|Settings|Scale|Max|GetScale_Y_Max)) (Math|Random|RandomFloatinRange (Variables|Settings|Scale|Min|GetScale_Z_Min) (Variables|Settings|Scale|Max|GetScale_Z_Max))))
  (Transformation|SetWorldRotation _staticmesh (Math|Rotator|MakeRotator (.roll _returnvalue) (.pitch _returnvalue) (Math|Random|RandomFloatinRange 0.0 3.6e+02)) false false))